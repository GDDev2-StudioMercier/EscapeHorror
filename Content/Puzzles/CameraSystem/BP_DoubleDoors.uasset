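; Double door actor in the camera system puzzle folder that swings both leaves open.
; BeginPlay caches the starting relative rotations of the Left and Right components.
; The Open event plays a timeline from the start, lerping each yaw 90 degrees from its cached value in opposite directions while keeping pitch and roll.
; The file contains no closing logic and no caller of Open.
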(event `self.ReceiveBeginPlay`
  (set `self.LeftRotation` (`SceneComponent.RelativeRotation` (`self.Left`)))
  (set `self.RightRotation` (`SceneComponent.RelativeRotation` (`self.Right`))))

(event `Open`
  (bind (_leftrotation_roll _leftrotation_pitch _leftrotation_yaw) (`KismetMathLibrary.BreakRotator` (`self.LeftRotation`)))
  (bind (_rightrotation_roll _rightrotation_pitch _rightrotation_yaw) (`KismetMathLibrary.BreakRotator` (`self.RightRotation`)))
  (bind (_direction _alpha) (`Timeline|Timeline` :!via `PlayFromStart`)
    (:`Update`
      (`SceneComponent.K2_SetRelativeRotation` (`self.Left`) (`KismetMathLibrary.MakeRotator` _leftrotation_roll _leftrotation_pitch (`KismetMathLibrary.Lerp` _leftrotation_yaw (+ _leftrotation_yaw 90.0) _alpha)) false false)
      (`SceneComponent.K2_SetRelativeRotation` (`self.Right`) (`KismetMathLibrary.MakeRotator` _rightrotation_roll _rightrotation_pitch (`KismetMathLibrary.Lerp` _rightrotation_yaw (- _rightrotation_yaw 90.0) _alpha)) false false))))

(fn `UserConstructionScript`)