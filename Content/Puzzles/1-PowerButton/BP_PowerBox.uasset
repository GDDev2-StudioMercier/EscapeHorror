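; BP_PowerBox is a puzzle power box whose handle opens a cell door when it receives the correct power value.
; InteractPlayer compares the incoming value to PowerNeeded with a small tolerance; a match turns the handle fully, opens CellDoorRef and closes a gate against further attempts.
; A mismatch plays the HandleAnimation timeline, easing the handle from an angle proportional to that value back to rest.
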(event `/Game/FirstPerson/Blueprints/BPI_Interact.Interact_Player`
  (params (PowerInteract :type "Float (double-precision)") (ComponentHit :type "PrimitiveComponent Object Reference"))
  (bind _handle (`self.Handle`))
  (`/Engine/EditorBlueprintResources/StandardMacros.Gate` false :!label _label
    (:`Exit`
      (if (`KismetMathLibrary.NearlyEqual_FloatFloat` PowerInteract (`self.PowerNeeded`) 0.01)
        (`|ExecutionSequence`
          (:`then_0`
            (`SceneComponent.K2_SetWorldRotation` _handle (`KismetMathLibrary.MakeRotator` 70.0) false false)
            (`/Game/Puzzles/1-PowerButton/BP_CellDoor.Open` (`self.CellDoorRef`)))
          (:`then_1`
            (goto _label :!via `Close`)))
        (else
          (bind (_direction _handlereturninginitialrotationlerp) (`Timeline|HandleAnimation` :!via `PlayFromStart`)
            (:`Update`
              (`SceneComponent.K2_SetWorldRotation` _handle (`KismetMathLibrary.MakeRotator` (`KismetMathLibrary.Lerp` (`KismetMathLibrary.Lerp` 0.0 70.0 PowerInteract) 0.0 _handlereturninginitialrotationlerp)) false false))))))))

(fn `UserConstructionScript`)