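; BP_ButtonOrder is a numbered switch in a button-order puzzle that the player can flip while DoorNotOpen is true.
; A timeline rolls the switch mesh 90 degrees from its starting rotation, playing or reversing according to IsOff.
; When it finishes, it toggles IsOff and passes its number and state to the button order manager for verification.
; A Reset event reverses the switch, and EmitSpark spawns an attached Niagara spark effect.
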(event `self.ReceiveBeginPlay`
  ; Begin Play
  (set `self.SwitchRotation` (`SceneComponent.RelativeRotation` (`self.Switch5`))))

(event `/Game/FirstPerson/Blueprints/BPI_Interact.Interact_Player`
  (params (PowerInteract :type "Float (double-precision)") (ComponentHit :type "PrimitiveComponent Object Reference"))
  (bind (_switchrotation_roll _switchrotation_pitch _switchrotation_yaw) (`KismetMathLibrary.BreakRotator` (`self.SwitchRotation`)))
  ; Interact
  (if (`self.DoorNotOpen`)
    (if (`self.IsOff`)
      (bind (_direction _alpha) (`Timeline|Rotation` :!label _label)
        (:`Update`
          (`SceneComponent.K2_SetRelativeRotation` (`self.Switch5`) (`KismetMathLibrary.MakeRotator` (`KismetMathLibrary.Lerp` _switchrotation_roll (+ _switchrotation_roll 90.0) _alpha) _switchrotation_pitch _switchrotation_yaw) false false))
        (:`Finished`
          (set `self.IsOff` (not (`self.IsOff`)))
          (`/Game/Puzzles/ButtonOrder/BP_ButtonOrderManager.VerifyCode` (`self.ButtonOrderManagerRef`) (`self.Number`) (`self.IsOff`))))
      (else
        (goto _label :!via `Reverse`)))))

(event `Reset`
  ; Interact
  (goto _label :!via `Reverse`))

(event `EmitSpark`
  ; Spawn Spark
  (`NiagaraFunctionLibrary.SpawnSystemAttached` "/Game/PolygonHorrorMansion/FX/Niagara/NS_Sparks_01.NS_Sparks_01" (`self.Scene`) "None" (0.0 0.0 0.0) (struct :`Yaw` -90.0) "KeepRelativeOffset" true))

(fn `UserConstructionScript`)