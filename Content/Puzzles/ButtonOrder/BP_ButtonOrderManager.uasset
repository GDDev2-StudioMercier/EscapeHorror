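; Puzzle manager that opens a door when five buttons are switched on in the order given by a code.
; A looping timer makes the buttons spark one after another in array order, pausing before each repeat.
; VerifyCode tracks the on count and appends pressed numbers to a string.
; At five on, it compares the last five characters to the code, then either opens the door or resets the buttons.
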(event `self.ReceiveBeginPlay`
  ; Begin Play
  (`self.Sparks`))

(event `Sparks`
  ; Spark Timer
  (bind _returnvalue (`KismetSystemLibrary.K2_SetTimerDelegate` (delegate `SparkTimer`) 0.75 true))
  (set `self.SparkTimerHandle` _returnvalue))

(event `SparkTimer`
  ; Spark Timer
  (`/Game/Puzzles/ButtonOrder/BP_ButtonOrder.EmitSpark` (`|GetArrayItem` (`self.ButtonsRef`) (`self.Index`)))
  (if (>= (`self.Index`) 4)
    (`self.SparkPause`)
    (else
      (`/Engine/EditorBlueprintResources/StandardMacros.IncrementInt` (`self.Index`)))))

(event `SparkPause`
  ; Spark Timer
  (if (`KismetSystemLibrary.K2_IsValidTimerHandle` (`self.SparkTimerHandle`))
    (`KismetSystemLibrary.K2_ClearAndInvalidateTimerHandle` (`self.SparkTimerHandle`))
    (set `self.Index` 0)
    (`KismetSystemLibrary.Delay` 3.0)
    (`self.Sparks`)))

(event `VerifyCode`
  (params (ButtonNumber :type String) (IsOff :type Boolean))
  (bind _currentcode (`self.CurrentCode`))
  (bind _returnvalue (`KismetStringLibrary.Len` _currentcode))
  ; Verify Code
  (set `self.Button Number` ButtonNumber)
  (set `self.AmmountOfButtonOn` (+ (`self.AmmountOfButtonOn`) (select `bool` IsOff :`false` 1 :`true` -1)))
  (set `self.CurrentCode` (`KismetStringLibrary.Concat_StrStr` (`self.CurrentCode`) (select `bool` IsOff :`false` (`self.Button Number`))))
  (if (== (`self.AmmountOfButtonOn`) 5)
    (if (`KismetStringLibrary.EqualEqual_StrStr` (`KismetStringLibrary.GetSubstring` _currentcode (- _returnvalue 5) _returnvalue) (`self.Code`))
      (`/Game/Puzzles/Misc/BP_Door.Open` (`self.DoorRef`))
      (for _array_element (`self.ButtonsRef`)
        (set `/Game/Puzzles/ButtonOrder/BP_ButtonOrder.DoorNotOpen` false _array_element))
      (else
        (for _array_element_2 (`self.ButtonsRef`)
          (`/Game/Puzzles/ButtonOrder/BP_ButtonOrder.Reset` _array_element_2))
        (set `self.CurrentCode` "")))))

(fn `UserConstructionScript`)