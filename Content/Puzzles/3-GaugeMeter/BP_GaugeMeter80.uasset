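; BP_GaugeMeter80 is a one-shot gauge puzzle actor that adds its "80" step to the gauge meter and can open the gauge door.
; Active80 passes a DoOnce into a Timeline that rolls the mesh and turns it red.
; Each Timeline update also calls Add80 on BP_GaugeMeter and runs the door check.
; That check opens BP_Door_gaugemeter when the first-person character's GaugemeterNumber equals 4.
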(event `active80`
  (bind _staticmesh (`self.StaticMesh`))
  (`/Engine/EditorBlueprintResources/StandardMacros.DoOnce` false
    (:`Completed`
      (bind (_direction _newtrack_0) (`Timeline|Timeline`)
        (:`Update`
          (`PrimitiveComponent.SetMaterial` _staticmesh 0 "/AnimationSharing/AnimSharingRed.AnimSharingRed")
          (`SceneComponent.K2_SetRelativeRotation` _staticmesh (`KismetMathLibrary.MakeRotator` _newtrack_0) false false)
          (bind _returnvalue (`GameplayStatics.GetActorOfClass` "/Game/Puzzles/3-GaugeMeter/BP_GaugeMeter.BP_GaugeMeter_C"))
          (`/Game/Puzzles/3-GaugeMeter/BP_GaugeMeter.add80` _returnvalue)
          (`self.open_door_gauge_80`))))))

(event `open_door_gauge_80`
  (bind _returnvalue (`GameplayStatics.GetActorOfClass` "/Game/FirstPerson/Blueprints/BP_FirstPersonCharacter.BP_FirstPersonCharacter_C"))
  (if (== (`/Game/FirstPerson/Blueprints/BP_FirstPersonCharacter.gaugemeter_number` _returnvalue) 4)
    (bind _returnvalue_2 (`GameplayStatics.GetActorOfClass` "/Game/Puzzles/3-GaugeMeter/BP_Door_gaugemeter.BP_Door_gaugemeter_C"))
    (`/Game/Puzzles/3-GaugeMeter/BP_Door_gaugemeter.open` _returnvalue_2)))

(fn `UserConstructionScript`)