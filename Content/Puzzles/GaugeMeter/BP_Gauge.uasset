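; BP_Gauge is a puzzle gauge that tracks a liquid level and opens a referenced door when it settles at a target amount.
; UpdateMeters adds or subtracts an amount based on an on/off flag, then triggers the level update.
; A timeline animates the normalized Level parameter on a dynamic material created in the construction script, then checks the target when finished.
; Once the door opens, further gauge animation and checks stop.
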(event `UpdateMeters`
  (params (AmmountOfLiquid :type "Float (double-precision)") (IsOff :type Boolean))
  ; Update Meters
  (set `self.NewMeter` (+ (`self.GaugeMeter`) (select `bool` IsOff :`false` (* AmmountOfLiquid -1) :`true` AmmountOfLiquid)))
  (set `self.OldMeter` (`self.GaugeMeter`))
  (set `self.GaugeMeter` (`self.NewMeter`))
  (`self.UpdateGaugeLevel` 0.0))

(event `UpdateGaugeLevel`
  (params (Alpha :type "Float (double-precision)"))
  ; Update Gauge Level
  (if (`self.DoorNotOpen`)
    (bind (_direction _alpha) (`Timeline|Timeline` :!via `PlayFromStart`)
      (:`Update`
        (`MaterialInstanceDynamic.SetScalarParameterValue` (`self.MaterialInstance`) "Level" (/ (`KismetMathLibrary.Lerp` (`self.OldMeter`) (`self.NewMeter`) _alpha) 400.0)))
      (:`Finished`
        (if (`KismetMathLibrary.NearlyEqual_FloatFloat` (`self.GaugeMeter`) 280.0)
          (`/Game/Puzzles/Misc/BP_Door.Open` (`self.DoorRef`))
          (set `self.DoorNotOpen` false))))))

(fn `UserConstructionScript`
  (bind _returnvalue (`KismetMaterialLibrary.CreateDynamicMaterialInstance` "/Game/Materials/M_Gauge.M_Gauge"))
  (bind _output_get (set `self.MaterialInstance` _returnvalue))
  (`PrimitiveComponent.SetMaterial` (`self.Gauge`) 0 _output_get))