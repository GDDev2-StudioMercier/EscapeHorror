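; Lever for a code puzzle that opens BP_Door_code_lever when the first-person character's LeverNumber equals 5.
; The Code event plays a Timeline that rolls the lever mesh, calling OpenDoor on every update to mark the lever active and test that number.
; A self-restarting random timer of up to five seconds re-triggers the Niagara spark effect from BeginPlay onward.
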(event `self.ReceiveBeginPlay`
  (`KismetSystemLibrary.K2_SetTimerDelegate` (delegate `sparkle`) (`KismetMathLibrary.RandomFloatInRange` 0.0 5.0) :!label _label))

(event `loop`
  (goto _label))

(event `sparkle`
  (`ActorComponent.Activate` (`self.NS_Sparks_01`) false)
  (`self.loop`))

(event `Code`
  (bind (_direction _newtrack_0) (`Timeline|Timeline` :!via `PlayFromStart`)
    (:`Update`
      (`SceneComponent.K2_SetRelativeRotation` (`self.StaticMesh1`) (`KismetMathLibrary.MakeRotator` _newtrack_0) false false)
      (`self.open door`))))

(event `open door`
  (set `self.lever_active?` true)
  (bind _returnvalue (`GameplayStatics.GetActorOfClass` "/Game/FirstPerson/Blueprints/BP_FirstPersonCharacter.BP_FirstPersonCharacter_C"))
  (if (== (`/Game/FirstPerson/Blueprints/BP_FirstPersonCharacter.lever number` _returnvalue) 5)
    (bind _returnvalue_2 (`GameplayStatics.GetActorOfClass` "/Game/Puzzles/2-Lever-Code/BP_Door_code_lever.BP_Door_code_lever_C"))
    (`/Game/Puzzles/2-Lever-Code/BP_Door_code_lever.open_lever_code` _returnvalue_2)))

(fn `UserConstructionScript`)