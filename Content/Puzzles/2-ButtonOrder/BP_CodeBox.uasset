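; BP_CodeBox is an interactable lever box in the button-order puzzle that toggles on and off when the player interacts.
; Each toggle reports its box number and new state to the code manager to add or remove it from the code.
; A timeline plays or reverses to swing the handle between rest and raised roll angles.
; ResetHandle switches the box off and returns the handle without notifying the manager.
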(event `/Game/FirstPerson/Blueprints/BPI_Interact.Interact_Player`
  (params (PowerInteract :type "Float (double-precision)") (ComponentHit :type "PrimitiveComponent Object Reference"))
  (if (`self.bActivated?`)
    (set `self.bActivated?` false)
    (`|ExecutionSequence`
      (:`then_0`
        (`/Game/Puzzles/2-ButtonOrder/BP_CodeBoxManager.ModifyCode` (`self.CodeManagerRef`) (`self.CodeBoxNumber`) (`self.bActivated?`) :!label _label))
      (:`then_1`
        (bind (_direction _rotationlerp) (`Timeline|HandleRotation` :!via `Reverse` :!label _label_2)
          (:`Update`
            (`SceneComponent.K2_SetRelativeRotation` (`self.Handle`) (`KismetMathLibrary.MakeRotator` (`KismetMathLibrary.Lerp` 0.0 70.0 _rotationlerp)) false false)))))
    (else
      (set `self.bActivated?` true)
      (`|ExecutionSequence`
        (:`then_0`
          (goto _label))
        (:`then_1`
          (goto _label_2))))))

(event `ResetHandle`
  (set `self.bActivated?` false)
  (goto _label_2 :!via `Reverse`))

(fn `UserConstructionScript`)