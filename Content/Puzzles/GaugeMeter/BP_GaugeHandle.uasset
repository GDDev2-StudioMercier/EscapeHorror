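; Interactable valve-style handle for a gauge puzzle that sends its liquid amount and off state to a referenced gauge meter.
; On interact, a DoOnce gates the meter update while a timeline spins the handle two full turns on roll, forward or in reverse depending on IsOff.
; The timeline also drives the Alpha parameter on a dynamic material, then flips IsOff and re-arms the DoOnce when finished.
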(event `self.ReceiveBeginPlay`
  ; Begin Play
  (set `self.HandleRotation` (`SceneComponent.RelativeRotation` (`self.Handle`))))

(event `/Game/FirstPerson/Blueprints/BPI_Interact.Interact_Player`
  (params (PowerInteract :type "Float (double-precision)") (ComponentHit :type "PrimitiveComponent Object Reference"))
  (bind (_handlerotation_roll _handlerotation_pitch _handlerotation_yaw) (`KismetMathLibrary.BreakRotator` (`self.HandleRotation`)))
  ; Interact Update Gauge Meter
  (`|ExecutionSequence`
    (:`then_0`
      (`/Engine/EditorBlueprintResources/StandardMacros.DoOnce` false :!label _label
        (:`Completed`
          (`/Game/Puzzles/GaugeMeter/BP_Gauge.UpdateMeters` (`self.GaugeRef`) (`self.AmmountOfLiquid`) (`self.IsOff`)))))
    (:`then_1`
      (if (`self.IsOff`)
        (bind (_direction _alpha) (`Timeline|Timeline` :!label _label_2)
          (:`Update`
            (`SceneComponent.K2_SetRelativeRotation` (`self.Handle`) (`KismetMathLibrary.MakeRotator` (`KismetMathLibrary.Lerp` _handlerotation_roll (- _handlerotation_roll 720.0) _alpha) _handlerotation_pitch _handlerotation_yaw) false false)
            (`MaterialInstanceDynamic.SetScalarParameterValue` (`self.MaterialInstance`) "Alpha" _alpha))
          (:`Finished`
            (set `self.IsOff` (not (`self.IsOff`)))
            (`self.Reset`)))
        (else
          (goto _label_2 :!via `Reverse`))))))

(event `Reset`
  ; Interact Update Gauge Meter
  (goto _label :!via `Reset`))

(fn `UserConstructionScript`
  (bind _returnvalue (`KismetMaterialLibrary.CreateDynamicMaterialInstance` "/Game/Materials/M_Default.M_Default"))
  (bind _output_get (set `self.MaterialInstance` _returnvalue))
  (`PrimitiveComponent.SetMaterial` (`self.Handle`) 0 _output_get))