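; BP_PowerButton is a puzzle power switch that opens a referenced door once the player fully engages it.
; The InteractPlayer event maps its PowerInteract value to the Switch component's roll, tilting it toward a fixed end angle.
; Reaching that angle calls Open on DoorRef through a DoOnce.
; Short of it, a retriggerable delay snaps the switch back to rest shortly after interaction calls stop.
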(event `/Game/FirstPerson/Blueprints/BPI_Interact.Interact_Player`
  (params (PowerInteract :type "Float (double-precision)") (ComponentHit :type "PrimitiveComponent Object Reference"))
  (bind _returnvalue (`KismetMathLibrary.Lerp` 0.0 60.0 PowerInteract))
  (bind _returnvalue_2 (== _returnvalue 60.0))
  ; Set Rotation
  (`SceneComponent.K2_SetRelativeRotation` (`self.Switch`) (`KismetMathLibrary.MakeRotator` _returnvalue) false false)
  (if _returnvalue_2
    (`/Engine/EditorBlueprintResources/StandardMacros.DoOnce` false
      (:`Completed`
        (`/Game/Puzzles/Misc/BP_Door.Open` (`self.DoorRef`))))
    (else
      (`KismetSystemLibrary.RetriggerableDelay` 0.1)
      (if (not _returnvalue_2)
        (`SceneComponent.K2_SetRelativeRotation` (`self.Switch`) (`KismetMathLibrary.MakeRotator` 0.0) false false)))))

(fn `UserConstructionScript`)