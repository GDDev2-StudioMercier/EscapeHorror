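; Interactable valve for the gauge meter puzzle that toggles a pressure contribution on or off.
; Each interaction flips ValveActivated and passes PressurePower with the new state to the referenced gauge meter.
; The ValveSpin timeline plays forward or in reverse, spinning the valve two turns and blending its dynamic material between white and red.
; A text component displays the valve's pressure value from BeginPlay.
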(event `self.ReceiveBeginPlay`
  (bind _returnvalue (`PrimitiveComponent.CreateDynamicMaterialInstance` (`self.Valve`) 0 "/Game/Puzzles/3-GaugeMeter/M_Valve.M_Valve" "None"))
  (set `self.ValveMaterial` _returnvalue)
  (`TextRenderComponent.K2_SetText` (`self.PressurePowerText`) (`KismetTextLibrary.Conv_IntToText` (`self.PressurePower`))))

(event `/Game/FirstPerson/Blueprints/BPI_Interact.Interact_Player`
  (params (PowerInteract :type "Float (double-precision)") (ComponentHit :type "PrimitiveComponent Object Reference"))
  (if (`self.bValveActivated?`)
    (set `self.bValveActivated?` false)
    (`|ExecutionSequence`
      (:`then_0`
        (`/Game/Puzzles/3-GaugeMeter/BP_GaugeMeter.PressureChange` (`self.GaugeMeterRef`) (`self.PressurePower`) (`self.bValveActivated?`) :!label _label))
      (:`then_1`
        (bind (_direction _spinning) (`Timeline|ValveSpin` :!via `Reverse` :!label _label_2)
          (:`Update`
            (`SceneComponent.K2_SetRelativeRotation` (`self.Valve`) (`KismetMathLibrary.MakeRotator` (`KismetMathLibrary.Lerp` 0.0 720.0 _spinning)) false false)
            (`MaterialInstanceDynamic.SetVectorParameterValue` (`self.ValveMaterial`) "ValveColor" (`KismetMathLibrary.LinearColorLerp` (make `LinearColor` 1.0 1.0 1.0 1.0) (make `LinearColor` 1.0 0.2 0.2 1.0) _spinning))))))
    (else
      (set `self.bValveActivated?` true)
      (`|ExecutionSequence`
        (:`then_0`
          (goto _label))
        (:`then_1`
          (goto _label_2))))))

(fn `UserConstructionScript`)