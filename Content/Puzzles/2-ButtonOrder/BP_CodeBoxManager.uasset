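; BP_CodeBoxManager runs the button-order puzzle, checking an entered code and opening a cell door when it is correct.
; ModifyCode adds or removes a number from the current code as inputs change.
; Once the code holds five numbers, it is compared to the correct sequence in order.
; A match opens the referenced cell door; a mismatch clears the code and resets the handle on every linked code box.
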(event `ModifyCode`
  (params (Number :type Integer) (`Adding/Removing` :type Boolean))
  (bind _currentcode (`self.CurrentCode`))
  (if `Adding/Removing`
    (`KismetArrayLibrary.Array_Add` _currentcode Number)
    (else
      (`KismetArrayLibrary.Array_RemoveItem` _currentcode Number)))
  (if (== (`KismetArrayLibrary.Array_Length` _currentcode) 5)
    (if (`KismetArrayLibrary.Array_Identical` (`self.CurrentCode`) (`self.CorrectCode`))
      (`/Game/Puzzles/1-PowerButton/BP_CellDoor.Open` (`self.CellDoorRef`))
      (else
        (`KismetArrayLibrary.Array_Clear` (`self.CurrentCode`))
        (for _array_element (`self.CodeBoxRefs`)
          (`/Game/Puzzles/2-ButtonOrder/BP_CodeBox.ResetHandle` _array_element))))))

(fn `UserConstructionScript`)