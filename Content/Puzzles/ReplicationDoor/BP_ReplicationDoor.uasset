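; BP_ReplicationDoor is a puzzle door that plays an unlock-and-open animation through Multicast and Client events.
; BeginPlay caches the initial relative transforms of the latch and door.
; Both Open events share one path that drops the padlock and handle with physics, then runs a timeline.
; Separate timeline alpha tracks rotate the latch, slide it aside and swing the door open from the cached values.
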(event `self.ReceiveBeginPlay`
  ; Begin Play
  (set `self.LatchLocation` (`SceneComponent.RelativeLocation` (`self.Latch`)))
  (set `self.LatchRotation` (`SceneComponent.RelativeRotation` (`self.Latch`)))
  (set `self.DoorRotation` (`SceneComponent.RelativeRotation` (`self.Door`))))

(event `Multicast_Open`
  (bind (_latchrotation_roll _latchrotation_pitch _latchrotation_yaw) (`KismetMathLibrary.BreakRotator` (`self.LatchRotation`)))
  (bind (_doorrotation_roll _doorrotation_pitch _doorrotation_yaw) (`KismetMathLibrary.BreakRotator` (`self.DoorRotation`)))
  (bind (_latchlocation_x _latchlocation_y _latchlocation_z) (`KismetMathLibrary.BreakVector` (`self.LatchLocation`)))
  ; Door Anim
  (`|ExecutionSequence` :!label _label
    (:`then_0`
      (`PrimitiveComponent.SetSimulatePhysics` (`self.Padlock`) true)
      (`PrimitiveComponent.SetSimulatePhysics` (`self.PadlockHandle`) true))
    (:`then_1`
      (bind (_direction _latchalpha _latchalpha2 _dooralpha) (`Timeline|Timeline` :!via `PlayFromStart`)
        (:`Update`
          (`SceneComponent.K2_SetRelativeRotation` (`self.Latch`) (`KismetMathLibrary.MakeRotator` (`KismetMathLibrary.Lerp` _latchrotation_roll (- _latchrotation_roll 90.0) _latchalpha) _latchrotation_pitch _latchrotation_yaw) false false)
          (`SceneComponent.K2_SetRelativeLocation` (`self.Latch`) (`KismetMathLibrary.MakeVector` (`KismetMathLibrary.Lerp` _latchlocation_x (- _latchlocation_x 8.0) _latchalpha2) _latchlocation_y _latchlocation_z) false false)
          (`SceneComponent.K2_SetRelativeRotation` (`self.Door`) (`KismetMathLibrary.MakeRotator` _doorrotation_roll _doorrotation_pitch (`KismetMathLibrary.Lerp` _doorrotation_yaw (- _doorrotation_yaw 110.0) _dooralpha)) false false))))))

(event `Client_Open`
  ; Door Anim
  (goto _label))

(fn `UserConstructionScript`)