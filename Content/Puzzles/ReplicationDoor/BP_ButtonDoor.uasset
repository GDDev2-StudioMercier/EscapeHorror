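; BP_ButtonDoor is a puzzle button that helps open a referenced replication door when two presses are counted.
; Player interaction splits on authority into server and client interact events.
; Each event uses a DoOnce to turn the button green and increment the door's pressed count.
; At two, the server path calls the door's MulticastOpen, while the client path calls ClientOpen.
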(event `/Game/FirstPerson/Blueprints/BPI_Interact.Interact_Player`
  (params (PowerInteract :type "Float (double-precision)") (ComponentHit :type "PrimitiveComponent Object Reference"))
  ; Authority Check
  (`/Engine/EditorBlueprintResources/ActorMacros.Switch Has Authority`
    (:`Authority`
      (`self.Server_Interact`))
    (:`Remote`
      (`self.Client_Interact`))))

(event `Server_Interact`
  ; Interacts
  (`/Engine/EditorBlueprintResources/StandardMacros.DoOnce` false
    (:`Completed`
      (`PrimitiveComponent.SetMaterial` (`self.Button`) 0 "/Game/Materials/MI_Green.MI_Green")
      (bind _result (`/Engine/EditorBlueprintResources/StandardMacros.IncrementInt` (`/Game/Puzzles/ReplicationDoor/BP_ReplicationDoor.AmmountOfButtonPressed` (`self.ReplicationDoorRef`)))
        (:`  `
          (if (== _result 2)
            (`/Game/Puzzles/ReplicationDoor/BP_ReplicationDoor.Multicast_Open` (`self.ReplicationDoorRef`))))))))

(event `Client_Interact`
  ; Interacts
  (`/Engine/EditorBlueprintResources/StandardMacros.DoOnce` false
    (:`Completed`
      (`PrimitiveComponent.SetMaterial` (`self.Button`) 0 "/Game/Materials/MI_Green.MI_Green")
      (bind _result (`/Engine/EditorBlueprintResources/StandardMacros.IncrementInt` (`/Game/Puzzles/ReplicationDoor/BP_ReplicationDoor.AmmountOfButtonPressed` (`self.ReplicationDoorRef`)))
        (:`  `
          (if (== _result 2)
            (`/Game/Puzzles/ReplicationDoor/BP_ReplicationDoor.Client_Open` (`self.ReplicationDoorRef`))))))))

(fn `UserConstructionScript`)